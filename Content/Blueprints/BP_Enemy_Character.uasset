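; Enemy character for a top-down shooter that chases the player, deals damage on reaching them and flashes when hurt.
; ChasePlayer runs AI MoveTo; success applies the enemy's Attack to the player's health bar component, then chases again after a delay.
; Its own health component's events drive a hit sound and timeline tint on dynamic materials, and on death remove it from its spawner and destroy it.
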(event OnTakeDamage(BP_TDShooter_HealthBarComponent)
  (Audio|PlaySound2D "/Game/Sounds/Hit2.Hit2" 1.0 1.0 0.0 0 0)
  (bind _damagecolor (Timeline|TakeDamage_Timeline PlayFromStart)
    (:Update
      (for _array_element (Variables|Default|GetDynamicMaterials)
        (Rendering|Material|SetVectorParameterValue _array_element "Tint" _damagecolor :!class /Script/Engine.MaterialInstanceDynamic)))))

(event OnDie(BP_TDShooter_HealthBarComponent)
  (Default|RemoveEnemy (Variables|Default|GetSpawner) self)
  (Actor|DestroyActor))

(event Custom|ChasePlayer
  (bind _movementresult (AI|AIMoveTo self "0, 0, 0" (Game|Player|GetPlayerPawn 0) 5.0 false)
    (:OnSuccess
      (CallFunction|DealDamage))
    (:OnFail
      (Development|PrintString (Utilities|String|EnumtoString _movementresult)))))

(event Custom|DealDamage
  (Class|TDShooterHealthBarComponent|TakeDamage (Actor|GetComponentbyClass (Game|Player|GetPlayerPawn 0) "/Game/Blueprints/BP_TDShooter_HealthBarComponent.BP_TDShooter_HealthBarComponent_C") (Variables|/Script/TDShooter.TDShooterHealthBarComponent|Getattack (Variables|Default|GetBP_TDShooter_HealthBarComponent)))
  (Utilities|FlowControl|Delay (Variables|Default|GetAfterHitDelay))
  (CallFunction|ChasePlayer))

(event EventBeginPlay
  (bind _dynamicmaterials (CallFunction|CreateDynamicMaterials (Variables|Character|GetMesh)))
  (Variables|Default|SetDynamicMaterials _dynamicmaterials))

(fn ConstructionScript)