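; BP_TDShooter_Character is a top-down shooter character that reacts to damage and death from its health bar component.
; BeginPlay creates dynamic materials on the mesh and tints them blue.
; Taking damage plays a hit sound and runs a timeline that animates the tint color across those materials.
; On death it plays a death sound, shows the lose screen widget and pauses the game.
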(event OnTakeDamage(BP_TDShooter_HealthBarComponent)
  (Audio|PlaySound2D "/Game/Sounds/Hit.Hit" 1.0 1.0 0.0 0 0)
  (bind _damagecolor (Timeline|TakeDamage_Timeline PlayFromStart)
    (:Update
      (for _array_element (Variables|Default|GetDynamicMaterials)
        (Rendering|Material|SetVectorParameterValue _array_element "Tint" _damagecolor :!class /Script/Engine.MaterialInstanceDynamic)))))

(event OnDie(BP_TDShooter_HealthBarComponent)
  (Audio|PlaySound2D "/Game/Sounds/PlayerDeath.PlayerDeath" 1.0 1.0 0.0 0 0)
  (bind _returnvalue (UserInterface|CreateWidget "/Game/Blueprints/WBP_LoseScreen.WBP_LoseScreen_C"))
  (UserInterface|Viewport|AddtoViewport _returnvalue 0)
  (Game|SetGamePaused true))

(event EventBeginPlay
  (bind _dynamicmaterials (CallFunction|CreateDynamicMaterials (Variables|Character|GetMesh)))
  (bind _output_get (Variables|Default|SetDynamicMaterials _dynamicmaterials))
  (for _array_element _output_get
    (Rendering|Material|SetVectorParameterValue _array_element "Tint" "(R=0.000000,G=0.500000,B=1.000000,A=1.000000)" :!class /Script/Engine.MaterialInstanceDynamic)))

(fn ConstructionScript)