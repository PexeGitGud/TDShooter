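; BP_TDShooter_Bullet is a shooter bullet that can ricochet from a damaged enemy toward another nearby one.
; On BeginPlay it caches the BP_EnemySpawner, whose EnemyArray supplies the candidate targets.
; Ricochet scans that array, skipping the damaged enemy, and keeps the position closest to the bullet in ClosestEnemy, which is never reset here.
; Unless that position matches a fixed sentinel vector, it zeroes the sphere's velocity and calls AddImpulse toward it at BulletSpeed.
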(event EventRicochet
  (params (DamagedActor :type Actor%20Object%20Reference))
  (bind _returnvalue (Transformation|GetActorLocation))
  (bind _asbp_enemy_character (Utilities|Casting|CastToBP_Enemy_Character DamagedActor))
  (for _array_element (Variables|/Game/Blueprints/BP_EnemySpawner.BP_EnemySpawner_C|GetEnemyArray (Variables|Default|GetEnemySpawner))
    (if (!= _asbp_enemy_character _array_element)
      (if (< (Math|Vector|Distance(Vector) (Transformation|GetActorLocation _array_element) _returnvalue) (Math|Vector|Distance(Vector) _returnvalue (Variables|Default|GetClosestEnemy)))
        (Variables|Default|SetClosestEnemy (Transformation|GetActorLocation _array_element)))))
  (if (Utilities|Operators|NotEqual(!=) (Variables|Default|GetClosestEnemy) "100.000000,100.000000,100.000000" 0.1)
    (Physics|SetPhysicsLinearVelocity (Variables|Default|GetSphere) "0, 0, 0" false "None")
    (Class|TDShooterBullet|AddImpulse (Math|Vector|Normalize (- (Variables|Default|GetClosestEnemy) (Transformation|GetActorLocation))) (Variables|Default|GetbulletSpeed))))

(event EventBeginPlay
  (bind _returnvalue (Actor|GetActorOfClass "/Game/Blueprints/BP_EnemySpawner.BP_EnemySpawner_C"))
  (Variables|Default|SetEnemySpawner _returnvalue))

(fn ConstructionScript)