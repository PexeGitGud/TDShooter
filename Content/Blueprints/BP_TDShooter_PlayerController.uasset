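; Player controller for the top-down shooter that toggles game pause from the IA_PauseGame input action.
; When that action completes, it checks the paused state, plays a matching UI blip sound and calls PauseGame or Unpause.
; PauseGame creates the WBP_PauseMenu widget if no valid one exists, then shows it and pauses the game.
; Unpause hides the widget and resumes play, keeping it for reuse.
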(event Custom|PauseGame
  (Utilities|IsValid (Variables|Default|GetPauseMenuWidget)
    (:Is%20Valid
      _)
    (:Is%20Not%20Valid
      (bind _returnvalue (UserInterface|CreateWidget "/Game/Blueprints/WBP_PauseMenu.WBP_PauseMenu_C"))
      (bind _output_get (Variables|Default|SetPauseMenuWidget _returnvalue))
      (UserInterface|Viewport|AddtoViewport _output_get 0)))
  (Widget|SetVisibility (Variables|Default|GetPauseMenuWidget) "Visible")
  (Game|SetGamePaused true))

(event Custom|Unpause
  (Widget|SetVisibility (Variables|Default|GetPauseMenuWidget) "Hidden")
  (Game|SetGamePaused false))

(event Input|EnhancedActionEvents|EnhancedInputActionIA_PauseGame
  (params (ActionValue :type Boolean) (ElapsedSeconds :type Float%20%28double-precision%29) (TriggeredSeconds :type Float%20%28double-precision%29) (InputAction :type Input%20Action%20Object%20Reference :default "/Game/Input/Actions/IA_PauseGame.IA_PauseGame"))
  (:Completed
    (if (Game|IsGamePaused)
      (Audio|PlaySound2D "/Game/Sounds/Blip_Select3.Blip_Select3" 1.0 1.0 0.0 0 0)
      (CallFunction|Unpause)
      (else
        (Audio|PlaySound2D "/Game/Sounds/Blip_Select2.Blip_Select2" 1.0 1.0 0.0 0 0)
        (CallFunction|PauseGame)))))

(fn ConstructionScript)