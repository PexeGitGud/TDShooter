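; BP_EnemySpawner keeps spawning enemy characters at random spawn points, up to a maximum number of tracked enemies.
; On BeginPlay it caches every BP_EnemySpawningPoint and starts a self-calling Delay loop paced by SpawnRate.
; While EnemyArray is below MaxEnemys, each tick of the loop spawns a BP_Enemy_Character, passes itself as Spawner and calls ChasePlayer.
; RemoveEnemy takes an enemy out of the array, freeing a slot.
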(event Custom|InstatiateEnemy
  (bind _self self)
  (bind _returnvalue (Game|SpawnActorfromClass "/Game/Blueprints/BP_Enemy_Character.BP_Enemy_Character_C" (Transformation|GetActorTransform (.OutItem (Utilities|Array|Random (Variables|Default|GetSpawningPoints)))) "AdjustIfPossibleButAlwaysSpawn" _self _self 0))
  (Utilities|Array|Add (Variables|Default|GetEnemyArray) _returnvalue)
  (Default|ChasePlayer _returnvalue))

(event Custom|SpawnEnemy
  (Utilities|FlowControl|Delay (Variables|Default|GetSpawnRate))
  (CallFunction|SpawnEnemy)
  (if (< (Utilities|Array|Length (Variables|Default|GetEnemyArray)) (Variables|Default|GetMaxEnemys))
    (CallFunction|InstatiateEnemy)))

(event Custom|RemoveEnemy
  (params (Enemy :type BP%20Enemy%20Character%20Object%20Reference%20%28by%20ref%29))
  (Utilities|Array|RemoveItem (Variables|Default|GetEnemyArray) Enemy))

(event EventBeginPlay
  (bind _outactors (Actor|GetAllActorsOfClass "/Game/Blueprints/BP_EnemySpawningPoint.BP_EnemySpawningPoint_C"))
  (Variables|Default|SetSpawningPoints _outactors)
  (CallFunction|SpawnEnemy))

(fn ConstructionScript)